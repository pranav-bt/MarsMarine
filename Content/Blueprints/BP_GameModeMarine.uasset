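; Wave-survival game mode that spawns escalating waves of BP_Alien enemies.
; Each wave multiplies the difficulty to set the alien count, then a looping timer spawns aliens at random TargetPoints until that count runs out.
; Spawned aliens are tracked in an array; RemoveAlienFromArray starts the next wave after a short delay once the array is empty and no spawns remain.
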(event Custom|Spawn%20Aliens
  (CallFunction|SpawningAliens))

(event Custom|End%20Wave
  (Utilities|FlowControl|Delay 3.0)
  (CallFunction|SetupNextWave))

(event EventBeginPlay
  (Utilities|FlowControl|Delay 2.0)
  (CallFunction|SetupNextWave))

(event EventTick
  (params (DeltaSeconds :type Float%20%28single-precision%29)))

(fn ConstructionScript)

(fn SetupNextWave
  (CallFunction|IncreaseDifficulty)
  (Math|Integer|IncrementInt (Variables|Default|GetCurrent%20Wave)
    (:%20%20
      (Utilities|Time|SetTimerbyFunctionName 0 "Spawn Aliens" 1.0 true))))

(fn GetRandomSpawnsPOints
  (bind _outactors (Actor|GetAllActorsOfClass "/Script/Engine.TargetPoint"))
  (return (Utilities|Array|Get(acopy) _outactors (Math|Random|RandomIntegerinRange 0 (Utilities|Array|LastIndex _outactors)))))

(fn SpawningAliens
  (bind _output (CallFunction|GetRandomSpawnsPOints))
  (Utilities|IsValid _output
    (:Is%20Valid
      (bind _returnvalue (Game|SpawnActorfromClass "/Game/Blueprints/BP_Alien.BP_Alien_C" (Transformation|GetActorTransform _output) "Undefined" 0 0))
      (Utilities|IsValid _returnvalue
        (:Is%20Valid
          (Utilities|Array|Add (Variables|Default|GetAliens) _returnvalue)
          (bind _result (Math|Integer|DecrementInt (Variables|Default|GetAlienSpawnNumber))
            (:%20%20
              (if (== _result 0)
                (Utilities|Time|ClearTimerbyFunctionName 0 "Spawn Aliens")))))))))

(fn RemoveAlienfromArray
  (params (Alien :type BP%20Alien%20Object%20Reference%20%28by%20ref%29))
  (Utilities|Array|RemoveItem (Variables|Default|GetAliens) Alien)
  (if (and (== (Utilities|Array|Length (Variables|Default|GetAliens)) 0) (== (Variables|Default|GetAlienSpawnNumber) 0))
    (CallFunction|EndWave)))

(fn IncreaseDifficulty
  (bind _output_get (Variables|Default|SetWave%20Difficulty (Math|Float|Round (* (Variables|Default|GetWave%20Difficulty) (Variables|Default|GetDifficulty%20Multiplier)))))
  (Variables|Default|SetAlienSpawnNumber _output_get))