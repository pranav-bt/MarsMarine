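; BP_Alien is an enemy that chases the player marine, attacks up close and can be killed.
; A loop re-issues AI MoveTo at the player controller while alive.
; Tick halts movement to play the attack montage when in range; damage is not applied here.
; Damage lowers Health; at exactly zero it stops, leaves the game mode's alien array, increments the marine's kills and destroys itself after a delay.
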(event EventBeginPlay
  (bind _asbp_marine (Utilities|Casting|CastToBP_Marine (Game|GetPlayerCharacter 0)))
  (if (CallFunction|IsAlive) :!label _label
    (Variables|Default|SetMarine _asbp_marine)
    (AI|AIMoveTo self "0, 0, 0" (Game|GetPlayerController 0) 5.0 false
      (:OnSuccess
        _)
      (:OnFail
        _))
    (Utilities|FlowControl|Delay 0.2)
    (goto _label)))

(event Collision|EventActorBeginOverlap
  (params (OtherActor :type Actor%20Object%20Reference)))

(event EventTick
  (params (DeltaSeconds :type Float%20%28single-precision%29))
  (if (Math|Boolean|ANDBoolean (CallFunction|IsWithinAttackRange) (not (CallFunction|Isattacking)) (CallFunction|IsAlive))
    (Components|Activation|Deactivate (Variables|Character|GetCharacterMovement))
    (Animation|Montage|PlayMontage (Variables|Character|GetMesh) "/Game/Characters/Enemy_Great_Spider/Animations/AlienAttackMontage.AlienAttackMontage"
      (:OnCompleted
        (Components|Activation|Activate (Variables|Character|GetCharacterMovement) false)))))

(event Game|Damage|EventAnyDamage
  (params (Damage :type Float%20%28single-precision%29) (DamageType :type Damage%20Type%20Object%20Reference) (InstigatedBy :type Controller%20Object%20Reference) (DamageCauser :type Actor%20Object%20Reference))
  (bind _marine (Variables|Default|GetMarine))
  (if (CallFunction|IsAlive)
    (CallFunction|AlienDamage Damage)
    (if (== (Variables|Default|GetHealth) 0.0)
      (CallFunction|KillAI)
      (bind _result (Math|Integer|IncrementInt (Variables|/Game/Blueprints/BP_Marine.BP_Marine_C|GetEnemies%20killed _marine))
        (:%20%20
          (Variables|/Game/Blueprints/BP_Marine.BP_Marine_C|SetEnemies%20killed _marine _result)
          (Utilities|FlowControl|Delay 2.0)
          (Actor|DestroyActor))))))

(fn ConstructionScript)

(fn IsWithinAttackRange
  (bind _asbp_marine (Utilities|Casting|CastToBP_Marine (Game|GetPlayerCharacter 0)))
  (return (< (Transformation|GetDistanceTo _asbp_marine) (Variables|Default|GetAttackRange))))

(fn Isattacking
  (return (Animation|Montage|MontageIsPlaying (Components|SkeletalMesh|GetAnimInstance (Variables|Character|GetMesh)) "/Game/Characters/Enemy_Great_Spider/Animations/AlienAttackMontage.AlienAttackMontage")))

(fn AlienDamage
  (params (B :type Float%20%28single-precision%29))
  (Variables|Default|SetHealth (- (Variables|Default|GetHealth) B)))

(fn KillAI
  (bind _charactermovement (Variables|Character|GetCharacterMovement))
  (Variables|Default|SetDead true)
  (Components|Movement|StopMovementImmediately _charactermovement)
  (Components|Activation|Deactivate _charactermovement)
  (bind _asbp_game_mode_marine (Utilities|Casting|CastToBP_GameModeMarine (Game|GetGameMode)))
  (Default|RemoveAlienfromArray _asbp_game_mode_marine self))

(fn IsAlive
  (return (not (Variables|Default|GetDead))))