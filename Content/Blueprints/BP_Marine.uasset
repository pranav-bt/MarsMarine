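; BP_Marine is the player character for a twin-stick shooter, creating its HUD on begin play.
; World-axis input moves it, while the right thumbstick, past a deadzone, smoothly rotates the control rotation toward the stick angle.
; Holding fire runs a looping timer of muzzle-socket line traces that apply damage and impact effects, alongside muzzle flash and audio.
; Damage lowers health; exactly zero marks it dead, stopping fire and blocking input actions.
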(event EventBeginPlay
  (bind _returnvalue (UserInterface|CreateWidget "/Game/Blueprints/Player_HUD.Player_HUD_C" 0 self))
  (UserInterface|Viewport|AddtoViewport _returnvalue 0))

(event EventTick
  (params (DeltaSeconds :type Float%20%28single-precision%29))
  (if (CallFunction|IsAlive)
    (CallFunction|PlayerRotation)))

(event Game|Damage|EventAnyDamage
  (params (Damage :type Float%20%28single-precision%29) (DamageType :type Damage%20Type%20Object%20Reference) (InstigatedBy :type Controller%20Object%20Reference) (DamageCauser :type Actor%20Object%20Reference))
  (bind _player_health (CallFunction|DamageHealth Damage))
  (if (== _player_health 0.0)
    (Variables|Default|SetDead true)
    (CallFunction|StopFire)))

(event Input|ActionEvents|InputActionWeaponFire
  (params (Key :type Key%20Structure :default "None"))
  (:Pressed
    (CallFunction|FireGun))
  (:Released
    (CallFunction|StopFire)))

(event Input|AxisEvents|InputAxisMoveForwards/Backwards
  (params (AxisValue :type Float%20%28single-precision%29))
  (if (CallFunction|IsAlive)
    (Pawn|Input|AddMovementInput "1.000000, 0, 0" AxisValue false)))

(event Input|AxisEvents|InputAxisMoveRight/Left
  (params (AxisValue :type Float%20%28single-precision%29))
  (if (CallFunction|IsAlive)
    (Pawn|Input|AddMovementInput "0,1.000000, 0" AxisValue false)))

(fn ConstructionScript)

(fn CheckDeadzone
  (return (> (Math|Vector2D|Vector2DLength (Math|Vector2D|MakeVector2D (Input|AxisValues|GetRightThumbstickUp) (Input|AxisValues|GetRightThumbstickRight))) (Variables|Default|GetDeadzone))))

(fn PlayerRotation
  (bind _returnvalue (Game|GetPlayerController 0))
  (if (CallFunction|CheckDeadzone)
    (Pawn|SetControlRotation _returnvalue (Math|Interpolation|RInterpTo (Pawn|GetControlRotation _returnvalue :!class /Script/Engine.Controller) (Math|Rotator|MakeRotator 0.0 0.0 (Class|KismetMathLibrary|DegAtan2 (Input|AxisValues|GetRightThumbstickRight) (Input|AxisValues|GetRightThumbstickUp))) (Utilities|Time|GetWorldDeltaSeconds) (Variables|Default|GetCharacter%20Rotation%20Speed)))))

(fn FireGun
  (if (CallFunction|IsAlive)
    (Components|Activation|Activate (Variables|Default|GetP_AssaultRifle_MF) false)
    (bind _returnvalue (Audio|SpawnSound2D "/Game/Sounds/Weapon_AssaultRifle/Stereo/FiringCue.FiringCue" 1.0 1.0 0.0 0))
    (Variables|Default|SetWeaponfiresound _returnvalue)
    (CallFunction|WeaponDamage)
    (Utilities|Time|SetTimerbyFunctionName self "Weapon Damage" (Variables|Default|GetWeapon%20Firerate) true)))

(fn StopFire
  (bind _weaponfiresound (Variables|Default|GetWeaponfiresound))
  (Components|Activation|Deactivate (Variables|Default|GetP_AssaultRifle_MF))
  (Utilities|IsValid _weaponfiresound
    (:Is%20Valid
      (Audio|Components|Audio|Stop _weaponfiresound)
      (Utilities|Time|ClearTimerbyFunctionName 0 "Weapon Damage")
      (if (CallFunction|IsAlive)
        (Audio|SpawnSound2D "/Game/Sounds/Weapon_AssaultRifle/Stereo/AssaultRifle_ShotEnd05_Stereo.AssaultRifle_ShotEnd05_Stereo" 1.0 1.0 0.0 0)))))

(fn DamageHealth
  (params (B :type Float%20%28single-precision%29))
  (bind _output_get (Variables|Default|SetHealth (- (Variables|Default|GetHealth) B)))
  (return _output_get))

(fn IsAlive
  (return (not (Variables|Default|GetDead))))

(fn WeaponDamage
  (bind _outhit (Collision|LineTraceByChannel (CallFunction|GetWeaponStartTrace) (CallFunction|GetWeaponEndTrace) "TraceTypeQuery1" false 0 "None"))
  (if (.bBlockingHit (Collision|BreakHitResult _outhit))
    (Game|Damage|ApplyDamage (.HitActor (Collision|BreakHitResult _outhit)) (Variables|Default|GetGun%20Damage%20Per%20hit) 0 0)
    (CallFunction|SpawnBulletCollisionEffects (.Location (Collision|BreakHitResult _outhit)))))

(fn GetWeaponStartTrace
  (return (Transformation|GetSocketLocation (Variables|Default|GetRifle) "Muzzleflash")))

(fn GetWeaponEndTrace
  (return (+ (CallFunction|GetWeaponStartTrace) (* (Math|Vector|GetForwardVector (Pawn|GetControlRotation :!class /Script/Engine.Pawn)) (Variables|Default|GetWeapon%20Range)))))

(fn SpawnBulletCollisionEffects
  (params (Hit%20Location :type Vector))
  (Effects|SpawnEmitteratLocation "/Game/Effects/Weapons/Impacts/P_AssaultRifle_IH.P_AssaultRifle_IH" Hit%20Location))

(fn KillPlayerInstantly
  (Game|Damage|ApplyDamage (Game|GetPlayerCharacter 0) 1e+02 0 0))